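; Lobby game mode that registers joining and leaving players with BP_GameInstance and places each joining player at a numbered player start.
; On PostLogin, the local player restarts at start "1", while each remote player increments a join counter whose value names their start.
; The counter resets to 1 when only one player state exists and is not decremented on logout.
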(event EventOnLogout
  (params (ExitingController :type Controller%20Object%20Reference))
  (bind _asbp_game_instance (Utilities|Casting|CastToBP_GameInstance (Game|GetGameInstance)))
  (Default|RemoveLobbyPlayer _asbp_game_instance))

(event EventPostLogin
  (params (NewPlayer :type Player%20Controller%20Object%20Reference))
  (bind _asbp_game_instance (Utilities|Casting|CastToBP_GameInstance (Game|GetGameInstance)))
  (Default|AddLobbyPlayer _asbp_game_instance)
  (Utilities|FlowControl|Sequence
    (:then_0
      (if (== (Class|GameplayStatics|GetNumPlayerStates) 1)
        (Variables|Default|SetRemotePlayersJoined 1)))
    (:then_1
      (Variables|Default|SetPostLoginPlayer NewPlayer)
      (if (Pawn|IsLocalPlayerController (Variables|Default|GetPostLoginPlayer))
        (Class|GameModeBase|RestartPlayeratPlayerStart (Variables|Default|GetPostLoginPlayer) (Class|GameModeBase|FindPlayerStart (Variables|Default|GetPostLoginPlayer) "1"))
        (else
          (bind _result (Math|Integer|IncrementInt (Variables|Default|GetRemotePlayersJoined))
            (:%20%20
              (Class|GameModeBase|RestartPlayeratPlayerStart (Variables|Default|GetPostLoginPlayer) (Class|GameModeBase|FindPlayerStart (Variables|Default|GetPostLoginPlayer) (Utilities|String|ToString(Integer) _result))))))))))

(fn ConstructionScript)