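; Lobby player controller that shows either the login screen or the lobby UI to the local player.
; On BeginPlay it sets UI-only input, caches BP_GameInstance and binds to its login-complete event.
; It then creates BP_UI_Lobby if the game instance reports logged in, otherwise BP_UI_Login.
; OnLoginComplete adds the lobby widget on success; it does not remove the login widget or handle failures.
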(event EventBeginPlay
  (if (Pawn|IsLocalPlayerController)
    (Input|SetInputModeUIOnly self 0 "DoNotLock" false)
    (bind _asbp_game_instance (Utilities|Casting|CastToBP_GameInstance (Game|GetGameInstance)))
    (Variables|Default|SetGameInstanceRef _asbp_game_instance)
    (Utilities|FlowControl|Sequence
      (:then_0
        (EventDispatchers|BindEventtoOnLoginComplete (Variables|Default|GetGameInstanceRef) (EventDispatchers|CreateEvent :!event OnLoginComplete)))
      (:then_1
        (if (Class|MGGameInstance|IsLoggedin (Variables|Default|GetGameInstanceRef))
          (bind _returnvalue (UserInterface|CreateWidget "/Game/MyContent/UI/BP_UI_Lobby.BP_UI_Lobby_C" self))
          (UserInterface|Viewport|AddtoPlayerScreen _returnvalue)
          (else
            (bind _returnvalue_2 (UserInterface|CreateWidget "/Game/MyContent/UI/BP_UI_Login.BP_UI_Login_C" self))
            (UserInterface|Viewport|AddtoPlayerScreen _returnvalue_2)))))))

(fn ConstructionScript)

(fn OnLoginComplete
  (params (success :type Boolean) (error :type String))
  (if success
    (bind _returnvalue (UserInterface|CreateWidget "/Game/MyContent/UI/BP_UI_Lobby.BP_UI_Lobby_C" self))
    (UserInterface|Viewport|AddtoPlayerScreen _returnvalue)))