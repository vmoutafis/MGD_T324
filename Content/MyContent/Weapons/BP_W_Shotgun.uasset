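; Shotgun weapon Blueprint that fires multiple hitscan pellets per shot, building on a parent weapon class.
; On the server, it runs one damaging line trace per pellet, collects the hit locations and starts the cooldown.
; It then assigns the batch to a replicated array and plays trace effects locally.
; The array's OnRep replays those effects on clients, so one replicated variable carries the whole spread.
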(fn ConstructionScript
  (|CallParentFunction))

(fn FiredonServer
  (if (> (Variables|Default|GetBulletsPerShot) 0)
    (for _index (range 0 (- (Variables|Default|GetBulletsPerShot) 1))
      (bind _lasthitlocation (CallFunction|ApplyLineTraceDamage "None" false))
      (Utilities|Array|Add (LocalVariables|GetLLastHitLocations) _lasthitlocation))
    (CallFunction|StartCooldown)
    (bind _output_get (Variables|Default|SetLastHitLocations (LocalVariables|GetLLastHitLocations)))
    (for _array_element _output_get
      (CallFunction|PlayTraceFX _array_element))))

(fn OnRepLastHitLocations
  (for _array_element (Variables|Default|GetLastHitLocations)
    (CallFunction|PlayTraceFX _array_element)))