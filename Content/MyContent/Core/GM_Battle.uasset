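; GM_Battle is the battle game mode, which places keys in the level and marks a special player.
; On BeginPlay with authority, it gathers all KeySpawner actors and spawns a Key at three randomly picked ones, removing each from the pool so none repeats.
; On PostLogin, it sets IsSpecial on the new player's BP_PlayerState when the player state count is one, flagging the first player to join.
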(event EventPostLogin
  (params (NewPlayer :type Player%20Controller%20Object%20Reference))
  (bind _asbp_player_state (Utilities|Casting|CastToBP_PlayerState (Variables|/Script/Engine.Controller|GetPlayerState NewPlayer)))
  (if (== (Class|GameplayStatics|GetNumPlayerStates) 1)
    (Variables|/Game/MyContent/Player/BP_PlayerState.BP_PlayerState_C|SetIsSpecial _asbp_player_state true)))

(event EventBeginPlay
  (Networking|SwitchHasAuthority
    (:Authority
      (bind _outactors (Actor|GetAllActorsOfClass "/Game/MyContent/KeySpawner.KeySpawner_C"))
      (Variables|Default|SetAllKeysSpawners _outactors)
      (for _index (range 0 2)
        (bind _output_get (Variables|Default|SetChosenKeySpawn (.OutItem (Utilities|Array|Random (Variables|Default|GetAllKeysSpawners)))))
        (Game|SpawnActorfromClass "/Game/MyContent/Key.Key_C" (Transformation|GetActorTransform _output_get) "Undefined" "MultiplyWithRoot" 0 0)
        (Utilities|Array|RemoveItem (Variables|Default|GetAllKeysSpawners) (Variables|Default|GetChosenKeySpawn))))))

(fn ConstructionScript)